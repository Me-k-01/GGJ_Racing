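; Player controller for a wheeled vehicle that sets up input and drives the speedometer HUD.
; On BeginPlay it adds the default Enhanced Input mapping context, creates the vehicle UI widget in metric mode, and caches the controlled pawn's vehicle movement component.
; Each Tick it pushes forward speed and current gear from that component to the HUD.
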(event `self.ReceiveBeginPlay`
  (`EnhancedInputSubsystemInterface.AddMappingContext` (subsystem `EnhancedInputLocalPlayerSubsystem`) "/Game/VehicleTemplate/Input/IMC_Default.IMC_Default" 0 (struct)) ; Adding the Input Mapping Context needed to trigger the proper Input Actions.
  (bind _returnvalue (`|CreateWidget` "/Game/Blueprints/VehicleUI.VehicleUI_C" self))
  (bind _output_get (set `self.VehicleHud` _returnvalue))
  (`UserWidget.AddToViewport` _output_get 0)
  (bind _aswheeled_vehicle_pawn (cast `WheeledVehiclePawn` (`self.K2_GetPawn`)))
  (set `self.Vehicle Movement Component` (`WheeledVehiclePawn.VehicleMovementComponent` _aswheeled_vehicle_pawn)))

(event `self.ReceiveTick`
  (params (DeltaSeconds :type "Float (single-precision)"))
  (`/Game/Blueprints/VehicleUI.UpdateSpeed` (`self.VehicleHud`) (`ChaosVehicleMovementComponent.GetForwardSpeed` (`self.Vehicle Movement Component`)))
  (`/Game/Blueprints/VehicleUI.UpdateGear` (`self.VehicleHud`) (`ChaosVehicleMovementComponent.GetCurrentGear` (`self.Vehicle Movement Component`))))

(fn `UserConstructionScript`)